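; Game mode for KnightGuy that creates local players and swaps their pawns between playable character and init pawn.
; On BeginPlay it caches all PlayerStarts and calls CreatePlayer until the player count exceeds three.
; SpawnCharacter and DespawnCharacter destroy the controller's current valid pawn, then spawn and possess a BP_KnightGuyCharacter or BP_KnightGuy_InitPawn respectively.
; Spawn transforms come from GetRandomSpawnPoint, intended to pick among the cached starts.
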(event `self.ReceiveBeginPlay`
  (bind _numberofplayers (`self.NumberOfPlayers`))
  (bind _outactors (`GameplayStatics.GetAllActorsOfClass` "/Script/Engine.PlayerStart"))
  (set `self.SpawnPoints` _outactors)
  (while (<= _numberofplayers 3)
    (set `self.NumberOfPlayers` (+ _numberofplayers 1))
    (`GameplayStatics.CreatePlayer` -1)))

(event `SpawnCharacter`
  (params (PlayerController :type "PlayerController Object Reference"))
  (bind _returnvalue (`Controller.K2_GetPawn` PlayerController))
  (`/Engine/EditorBlueprintResources/StandardMacros.IsValid` _returnvalue
    (:`Is Valid`
      (`self.K2_DestroyActor` _returnvalue)
      (bind _returnvalue_2 (`|SpawnActorFromClass` "/Game/KnightGuy/Core/BP_KnightGuyCharacter.BP_KnightGuyCharacter_C" (`self.GetRandomSpawnPoint`) "Undefined" "OverrideRootScale" null null))
      (`Controller.Possess` PlayerController _returnvalue_2))))

(event `DespawnCharacter`
  (params (PlayerController :type "PlayerController Object Reference"))
  (bind _returnvalue (`Controller.K2_GetPawn` PlayerController))
  (`/Engine/EditorBlueprintResources/StandardMacros.IsValid` _returnvalue
    (:`Is Valid`
      (`self.K2_DestroyActor` _returnvalue)
      (bind _returnvalue_2 (`|SpawnActorFromClass` "/Game/KnightGuy/Core/BP_KnightGuy_InitPawn.BP_KnightGuy_InitPawn_C" (`self.GetRandomSpawnPoint`) "Undefined" "OverrideRootScale" null null))
      (`Controller.Possess` PlayerController _returnvalue_2))))

(fn `UserConstructionScript`)