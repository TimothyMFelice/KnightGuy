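; Base character Blueprint for KnightGuy that exposes melee, magic and potion actions on top of gameplay abilities.
; Light and heavy attacks both activate the current weapon slot's abilities, magic activates by tags and fires a magic-attack call, and potions use item slot zero.
; Attacks and magic require being alive, unpaused and not casting; attacks also block during active melee abilities, detected through tag queries.
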(fn `CanUseAnyAbility`
  (returns (Return :type Boolean))
  (return (and (`self.IsAlive`) (not (`GameplayStatics.IsGamePaused`)) (not (`self.Is Using Magic`)))))

(fn `DoHeavyAttack`
  (returns (Return :type Boolean))
  (if (and (`self.CanUseAnyAbility`) (not (`self.IsUsingAttack`)))
    (bind _returnvalue (`self.ActivateAbilitiesWithItemSlot` (`self.CurrentWeaponSlot`)))
    (return _returnvalue)))

(fn `DoLightAttack`
  (returns (Return :type Boolean))
  (if (and (`self.CanUseAnyAbility`) (not (`self.IsUsingAttack`)))
    (bind _returnvalue (`self.ActivateAbilitiesWithItemSlot` (`self.CurrentWeaponSlot`)))
    (return _returnvalue)))

(fn `DoMagic`
  (returns (Return :type Boolean))
  (if (`self.CanUseAnyAbility`)
    (bind _returnvalue (`self.ActivateAbilitiesWithTags` (struct)))
    (`self.OnMagicAttack`)
    (return _returnvalue)))

(fn `Is Using Magic`
  (returns (Return :type Boolean))
  (bind _activeabilities (`self.GetActiveAbilitiesWithTags` (struct :`GameplayTags` (struct :`(TagName` "Ability.Magic")))))
  (return (> (`KismetArrayLibrary.Array_Length` _activeabilities) 0)))

(fn `IsAlive`
  (returns (Return :type Boolean))
  (return (> (`self.GetHealth`) 0.0)))

(fn `IsUsingAttack`
  (returns (Return :type Boolean))
  (bind _activeabilities (`self.GetActiveAbilitiesWithTags` (struct :`GameplayTags` (struct :`(TagName` "Ability.Melee")))))
  (return (> (`KismetArrayLibrary.Array_Length` _activeabilities) 0)))

(fn `UseItemPotion`
  (`self.ActivateAbilitiesWithItemSlot` (make `KGItemSlot` "Potion" 0)))

(fn `UserConstructionScript`)