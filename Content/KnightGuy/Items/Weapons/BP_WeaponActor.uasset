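; BP_WeaponActor is a weapon actor that detects hits during attacks through a capsule overlap enabled only while an attack is active.
; A hit on an actor of a different class from the instigator sends the attack's gameplay event tag and target to the instigator, gated by a DoOnce that resets shortly after overlap ends.
; Hits also remove consumable weapons from inventory and trigger a count-limited hit pause using brief global time dilation.
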(event `self.ReceiveBeginPlay`
  (`PrimitiveComponent.IgnoreActorWhenMoving` (`self.Capsule`) null false))

(event `BeginWeaponAttack`
  (params (EventTag :type "GameplayTag Structure") (AttackDelayTime :type "Float (double-precision)") (AttackDelayCount :type Integer))
  (set `self.AttackEventTag` EventTag)
  (set `self.AttackDelayTime` AttackDelayTime)
  (set `self.AttackDelayCount` AttackDelayCount)
  (set `self.bIsAttacking` true)
  (`PrimitiveComponent.SetCollisionEnabled` (`self.Capsule`) "QueryOnly"))

(event `EndWeaponAttack`
  (set `self.bIsAttacking` false)
  (`PrimitiveComponent.SetCollisionEnabled` (`self.Capsule`) "NoCollision"))

(event `HitPause`
  (if (and (> (`self.AttackDelayCount`) 0) (`self.bEnableAttackDelay`))
    (`/Engine/EditorBlueprintResources/StandardMacros.DecrementInt` (`self.AttackDelayCount`)
      (:`  `
        (`KismetSystemLibrary.Delay` 0.1)
        (`GameplayStatics.SetGlobalTimeDilation` 0.1)
        (`KismetSystemLibrary.Delay` 0.01)
        (`GameplayStatics.SetGlobalTimeDilation` 1.0)))))

(event `self.ReceiveActorBeginOverlap`
  (params (OtherActor :type "Actor Object Reference"))
  (bind _returnvalue (`self.GetInstigator`))
  (if (and (!= (`GameplayStatics.GetObjectClass` OtherActor) (`GameplayStatics.GetObjectClass` (`self.GetInstigator`))) (`self.bIsAttacking`))
    (`/Engine/EditorBlueprintResources/StandardMacros.DoOnce` false :!label _label
      (:`Completed`
        (`AbilitySystemBlueprintLibrary.SendGameplayEventToActor` _returnvalue (`self.AttackEventTag`) (make `GameplayEventData` (struct) _returnvalue OtherActor))
        (`self.ConsumeWeapon`)
        (`self.HitPause`)))))

(event `self.ReceiveActorEndOverlap`
  (params (OtherActor :type "Actor Object Reference"))
  (`KismetSystemLibrary.Delay` 0.2)
  (goto _label :!via `Reset`))

(event `ConsumeWeapon`
  (bind _kgweaponitem (`self.KGWeaponItem`))
  (`/Engine/EditorBlueprintResources/StandardMacros.IsValid` _kgweaponitem
    (:`Is Valid`
      (if (`KGItem.IsConsumable` _kgweaponitem)
        (`KGPlayerControllerBase.RemoveInventoryItem` (`/Game/KnightGuy/Core/BP_KGFunctionLibrary.GetPlayerControllerBP`) (`self.KGWeaponItem`) 1)
        (if (< (`KGPlayerControllerBase.GetInventoryItemCount` (`/Game/KnightGuy/Core/BP_KGFunctionLibrary.GetPlayerControllerBP`) (`self.KGWeaponItem`)) 2)
          _)))))

(fn `UserConstructionScript`)