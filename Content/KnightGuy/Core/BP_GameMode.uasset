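; Game mode for KnightGuy that swaps a player controller between an init pawn and the knight character.
; On BeginPlay it caches all PlayerStart actors as spawn points.
; Spawn and despawn events destroy the currently controlled pawn, then spawn and possess the replacement at a transform from GetRandomSpawnPoint.
; A CreatePlayers helper adds local players in a counter loop, but nothing in this Blueprint calls it.
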(event `self.ReceiveBeginPlay`
  (`self.CacheVariables`))

(event `SpawnCharacter`
  (params (PlayerController :type "PlayerController Object Reference"))
  (bind _returnvalue (`Controller.K2_GetPawn` PlayerController))
  (`/Engine/EditorBlueprintResources/StandardMacros.IsValid` _returnvalue
    (:`Is Valid`
      (`self.K2_DestroyActor` _returnvalue)
      (bind _returnvalue_2 (`|SpawnActorFromClass` "/Game/KnightGuy/Core/BP_KnightGuy_Character.BP_KnightGuy_Character_C" (`self.GetRandomSpawnPoint`) "AlwaysSpawn" "OverrideRootScale" null null))
      (`Controller.Possess` PlayerController _returnvalue_2))))

(event `DespawnCharacter`
  (params (PlayerController :type "PlayerController Object Reference"))
  (bind _returnvalue (`Controller.K2_GetPawn` PlayerController))
  (`/Engine/EditorBlueprintResources/StandardMacros.IsValid` _returnvalue
    (:`Is Valid`
      (`self.K2_DestroyActor` _returnvalue)
      (bind _returnvalue_2 (`|SpawnActorFromClass` "/Game/KnightGuy/Core/BP_Pawn_Init.BP_Pawn_Init_C" (`self.GetRandomSpawnPoint`) "Undefined" "OverrideRootScale" null null))
      (`Controller.Possess` PlayerController _returnvalue_2))))

(fn `CacheVariables`
  (bind _outactors (`GameplayStatics.GetAllActorsOfClass` "/Script/Engine.PlayerStart"))
  (set `self.SpawnPoints` _outactors))

(fn `CreatePlayers`
  (bind _numberofplayers (`self.NumberOfPlayers`))
  (while (<= _numberofplayers 3)
    (set `self.NumberOfPlayers` (+ _numberofplayers 1))
    (`GameplayStatics.CreatePlayer` -1)))

(fn `UserConstructionScript`)