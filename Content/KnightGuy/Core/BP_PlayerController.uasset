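; Player controller for KnightGuy that sets up the knight character on possession and toggles spawning through the Pause input.
; First possession caches the BP_KnightGuy_Character, creates its weapons, unbinds an inventory-change delegate and sets game-only input.
; Pause presses alternate between asking BP_GameMode to spawn and despawn this controller's character.
; HUD creation and the inventory-change handler are empty stubs.
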(event `self.ReceivePossess`
  (params (PossessedPawn :type "Pawn Object Reference"))
  (`/Engine/EditorBlueprintResources/StandardMacros.DoOnce` false
    (:`Completed`
      (bind _asbp_knight_guy_character (cast `/Game/KnightGuy/Core/BP_KnightGuy_Character` PossessedPawn))
      (set `self.PlayerCharacter` _asbp_knight_guy_character)
      (`self.CreateHUD`)
      (remove `self.OnInventoryItemChanged` (`|CreateDelegate` :!event `EventInventoryItemChanged`))
      (`/Game/KnightGuy/Core/BP_KnightGuy_Character.CreateAllWeapons` (`self.PlayerCharacter`))
      (`WidgetBlueprintLibrary.SetInputMode_GameOnly` self))))

(event `CreateHUD`)

(event `InputAction|Pause`
  (params (Key :type "Key Structure"))
  (:`Pressed`
    (`/Engine/EditorBlueprintResources/StandardMacros.FlipFlop`
      (:`A`
        (bind _asbp_game_mode (cast `/Game/KnightGuy/Core/BP_GameMode` (`GameplayStatics.GetGameMode`)))
        (`/Game/KnightGuy/Core/BP_GameMode.SpawnCharacter` _asbp_game_mode self))
      (:`B`
        (bind _asbp_game_mode_2 (cast `/Game/KnightGuy/Core/BP_GameMode` (`GameplayStatics.GetGameMode`)))
        (`/Game/KnightGuy/Core/BP_GameMode.DespawnCharacter` _asbp_game_mode_2 self)))))

(event `EventInventoryItemChanged`
  (params (bAdded :type Boolean) (Item :type "KGItem Object Reference")))

(fn `UserConstructionScript`)